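; Gameplay ability for the second attack in a combo, playing a montage and managing its combo input window through gameplay tags.
; After commit, it waits on window open and end gameplay events alongside the montage.
; Opening swaps Combo1Tag for ComboWindowTag as non-replicated loose tags on the avatar.
; Closing removes the window tag and ends the ability, as does montage completion, with debug prints tracing the stages.
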(event `self.K2_ActivateAbility`
  (`self.K2_CommitAbility`)
  (`AbilityTask_PlayMontageAndWait.CreatePlayMontageAndWaitProxy` "None" (`self.Montage to Play`)
    (:`then`
      (`AbilityTask_WaitGameplayEvent.WaitGameplayEvent` (struct :`TagName` "Event.ComboWindowOpen") null
        (:`then`
          (`AbilityTask_WaitGameplayEvent.WaitGameplayEvent` (struct :`TagName` "Event.ComboWindowEnd") null
            (:`EventReceived`
              (`KismetSystemLibrary.PrintString` "Combo2WindowClosed")
              (`AbilitySystemBlueprintLibrary.RemoveLooseGameplayTags` (`self.GetAvatarActorFromActorInfo`) (`self.ComboWindowTag`))
              (`self.K2_EndAbility`))))
        (:`EventReceived`
          (`KismetSystemLibrary.PrintString` "Combo2WindowOpen")
          (`AbilitySystemBlueprintLibrary.RemoveLooseGameplayTags` (`self.GetAvatarActorFromActorInfo`) (`self.Combo1Tag`))
          (`AbilitySystemBlueprintLibrary.AddLooseGameplayTags` (`self.GetAvatarActorFromActorInfo`) (`self.ComboWindowTag`)))))
    (:`OnCompleted`
      (`self.K2_EndAbility`))))

(event `self.K2_OnEndAbility`
  (params (bWasCancelled :type Boolean))
  (`KismetSystemLibrary.PrintString` "Combo2Ended"))